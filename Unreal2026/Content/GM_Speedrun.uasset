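; Speedrun game mode, judging by its name, that tracks level time and a coin count.
; While NivelTerminado is false, Tick adds world delta seconds to TiempoActual and prints it on every frame.
; The SumarMoneda event increments MonedasActuales by one when called.
; NivelTerminado is only read here, and BeginPlay and the construction script are empty.
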(event Custom|SumarMoneda
  (Variables|Default|SetMonedasActuales (+ (Variables|Default|GetMonedasActuales) 1)))

(event EventBeginPlay)

(event EventTick
  (params (DeltaSeconds :type Float%20%28single-precision%29))
  (if (not (Variables|Default|GetNivelTerminado))
    (bind _output_get (Variables|Default|SetTiempoActual (+ (Variables|Default|GetTiempoActual) (Utilities|Time|GetWorldDeltaSeconds))))
    (Development|PrintString (Utilities|String|ToString(Float) _output_get))))

(fn ConstructionScript)