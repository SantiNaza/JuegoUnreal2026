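; BP_WinZone is the level-completion trigger for a speedrun game.
; When the first-person character overlaps its Box, it reads the collected coin count from the GM_Speedrun game mode.
; With enough coins it sets the level-finished flag on the game mode and prints the elapsed time; otherwise it prints a missing-coins message.
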(event OnComponentBeginOverlap(Box)
  (params (OverlappedComponent :type Primitive%20Component%20Object%20Reference) (OtherActor :type Actor%20Object%20Reference) (OtherComp :type Primitive%20Component%20Object%20Reference) (OtherBodyIndex :type Integer) (bFromSweep :type Boolean) (SweepResult :type Hit%20Result%20Structure%20%28by%20ref%29))
  (Utilities|Casting|CastToBP_FirstPersonCharacter OtherActor)
  (bind _asgm_speedrun (Utilities|Casting|CastToGM_Speedrun (Game|GetGameMode)))
  (if (>= (Variables|/Game/GM_Speedrun.GM_Speedrun_C|GetMonedasActuales _asgm_speedrun) 3)
    (Variables|/Game/GM_Speedrun.GM_Speedrun_C|SetNivelTerminado _asgm_speedrun true)
    (Development|PrintString (Utilities|String|Append "¡Nivel Completado! Tiiempo: " (Utilities|String|ToString(Float) (Variables|/Game/GM_Speedrun.GM_Speedrun_C|GetTiempoActual _asgm_speedrun))))
    (else
      (Development|PrintString "FALTAN MONEDAS"))))

(event EventBeginPlay)

(event Collision|EventActorBeginOverlap
  (params (OtherActor :type Actor%20Object%20Reference)))

(event EventTick
  (params (DeltaSeconds :type Float%20%28single-precision%29)))

(fn ConstructionScript)