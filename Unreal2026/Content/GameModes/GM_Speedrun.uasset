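; GM_Speedrun is the game mode for a speedrun level, tracking elapsed time, coins collected and the victory screen.
; BeginPlay creates the WBP_UI widget, passing it the next level from BP_WinZone.
; Tick updates the timer from game time while NivelTerminado is false, and SumarMoneda increments the coin count.
; Victoria sets the destination level, reveals the win message and buttons, pauses the game and switches input to UI-only with the cursor shown.
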(event Custom|Victoria
  (params (destino :type Name))
  (bind _returnvalue (Game|GetPlayerController 0))
  (bind _ref_ui (Variables|Default|GetRef_UI))
  (Variables|/Game/UI/WBP_UI.WBP_UI_C|SetSiguienteNivel _ref_ui destino)
  ;[0.15 0.15 0.15 0.5] Mostrar pantalla de victoria
  (Widget|SetVisibility (Variables|/Game/UI/WBP_UI.WBP_UI_C|GetGanaste _ref_ui) "Visible")
  (Widget|SetVisibility (Variables|/Game/UI/WBP_UI.WBP_UI_C|GetButton_R _ref_ui) "Visible")
  (Widget|SetVisibility (Variables|/Game/UI/WBP_UI.WBP_UI_C|GetButton_S _ref_ui) "Visible")
  (Widget|SetVisibility (Variables|/Game/UI/WBP_UI.WBP_UI_C|GetButton_Exit _ref_ui) "Visible")
  (Game|SetGamePaused true)
  (Variables|/Script/Engine.PlayerController|SetbShowMouseCursor _returnvalue true)
  (Input|SetInputModeUIOnly _returnvalue 0 "DoNotLock" false))

(event Custom|SumarMoneda
  (Variables|Default|SetMonedasActuales (+ (Variables|Default|GetMonedasActuales) 1)))

(event EventBeginPlay
  (Variables|Default|SetTiempodeInicio 0.0)
  (bind _returnvalue (Actor|GetActorOfClass "/Game/BP_Objetos/BP_WinZone.BP_WinZone_C"))
  (bind _returnvalue_2 (UserInterface|CreateWidget "/Game/UI/WBP_UI.WBP_UI_C" 0 (Variables|/Game/BP_Objetos/BP_WinZone.BP_WinZone_C|GetNivelDestino _returnvalue)))
  (bind _output_get (Variables|Default|SetRef_UI _returnvalue_2))
  (UserInterface|Viewport|AddtoViewport _output_get 0))

(event EventTick
  (params (DeltaSeconds :type Float%20%28single-precision%29))
  (if (not (Variables|Default|GetNivelTerminado))
    (Variables|Default|SetTiempoActual (- (Utilities|Time|GetTimeSeconds) (Variables|Default|GetTiempodeInicio)))))

(fn ConstructionScript)