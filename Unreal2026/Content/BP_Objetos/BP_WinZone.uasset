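; BP_WinZone is the level-finish trigger of a speedrun mode, acting when BP_PlayerFerxo overlaps its box.
; With at least three coins in GM_Speedrun, it calls Victoria with the destination level; otherwise it prints a missing-coins message.
; After that call, it loads or creates a BP_SaveRanking save, appends the player's name from GI_Speedrun and the current time, then saves it.
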(event OnComponentBeginOverlap(Box)
  (params (OverlappedComponent :type Primitive%20Component%20Object%20Reference) (OtherActor :type Actor%20Object%20Reference) (OtherComp :type Primitive%20Component%20Object%20Reference) (OtherBodyIndex :type Integer) (bFromSweep :type Boolean) (SweepResult :type Hit%20Result%20Structure%20%28by%20ref%29))
  (Utilities|Casting|CastToBP_PlayerFerxo OtherActor)
  (bind _asgm_speedrun (Utilities|Casting|CastToGM_Speedrun (Game|GetGameMode)))
  (if (>= (Variables|/Game/GameModes/GM_Speedrun.GM_Speedrun_C|GetMonedasActuales _asgm_speedrun) 3)
    (Utilities|FlowControl|Sequence
      (:then_0
        (bind _asgm_speedrun_2 (Utilities|Casting|CastToGM_Speedrun (Game|GetGameMode)))
        (Default|Victoria _asgm_speedrun_2 (Variables|Default|GetNivelDestino)))
      (:then_1
        ;[0.15 0.15 0.15 0.5] Sistema de guardado de tiempo
        (bind _returnvalue (SaveGame|DoesSaveGameExist "Ranking3"))
        (if _returnvalue
          (bind _returnvalue_2 (SaveGame|LoadGamefromSlot "Ranking3"))
          (bind _asbp_save_ranking (Utilities|Casting|CastToBP_SaveRanking _returnvalue_2))
          (Variables|Default|SetSaveGame_Ref _asbp_save_ranking)
          (else
            (bind _returnvalue_3 (SaveGame|CreateSaveGameObject "/Game/SaveGame/BP_SaveRanking.BP_SaveRanking_C"))
            (Variables|Default|SetSaveGame_Ref _returnvalue_3)))
        (Utilities|Array|Add (Variables|/Game/SaveGame/BP_SaveRanking.BP_SaveRanking_C|GetListaDeTiempos (Variables|Default|GetSaveGame_Ref)) (Utilities|Struct|MakeST_Record (Variables|/Game/SaveGame/GI_Speedrun.GI_Speedrun_C|GetNombreJugador (.AsGI%20Speedrun (Utilities|Casting|CastToGI_Speedrun (Game|GetGameInstance)))) (Variables|/Game/GameModes/GM_Speedrun.GM_Speedrun_C|GetTiempoActual (.AsGM%20Speedrun (Utilities|Casting|CastToGM_Speedrun (Game|GetGameMode))))))
        (SaveGame|SaveGametoSlot (Variables|Default|GetSaveGame_Ref) "Ranking3")
        (Development|PrintString "SAVED")))
    (else
      (Development|PrintString "FALTAN MONEDAS"))))

(event EventBeginPlay)

(event Collision|EventActorBeginOverlap
  (params (OtherActor :type Actor%20Object%20Reference)))

(event EventTick
  (params (DeltaSeconds :type Float%20%28single-precision%29)))

(fn ConstructionScript)